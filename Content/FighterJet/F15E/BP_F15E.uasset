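; BP_F15E is the player-flown F-15E fighter jet, translating input into flight and ground controls.
; Pitch, roll, yaw, thruster, toggled flaps, wheel steering, braking and landing gear retraction all feed AeroPhysicsComponent.
; Separate look axes drive controller pitch and yaw.
; On BeginPlay it creates a Fighter widget for the first player, passes itself as a reference and adds it to the viewport.
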(event `InputAxis|LookUp`
  (params (AxisValue :type "Float (single-precision)"))
  (`self.AddControllerPitchInput` AxisValue))

(event `InputAxis|Pitch`
  (params (AxisValue :type "Float (single-precision)"))
  (`AeroPhysicsComponent.SetAeroPitchControl` (`self.AeroPhysicsComponent`) AxisValue))

(event `InputAxis|TurnRight`
  (params (AxisValue :type "Float (single-precision)"))
  (`self.AddControllerYawInput` AxisValue))

(event `InputAxis|Roll`
  (params (AxisValue :type "Float (single-precision)"))
  (`AeroPhysicsComponent.SetAeroRollControl` (`self.AeroPhysicsComponent`) AxisValue))

(event `InputAxis|WheelTurn`
  (params (AxisValue :type "Float (single-precision)"))
  (`AeroPhysicsComponent.SetSteeringWheels` (`self.AeroPhysicsComponent`) AxisValue))

(event `InputAxis|Yaw`
  (params (AxisValue :type "Float (single-precision)"))
  (`AeroPhysicsComponent.SetAeroYawControl` (`self.AeroPhysicsComponent`) AxisValue))

(event `InputAxis|Brake`
  (params (AxisValue :type "Float (single-precision)"))
  (`AeroPhysicsComponent.SetWheelsBrake` (`self.AeroPhysicsComponent`) AxisValue))

(event `InputAction|Flap`
  (params (Key :type "Key Structure"))
  (bind _aerophysicscomponent (`self.AeroPhysicsComponent`))
  (:`Pressed`
    (`/Engine/EditorBlueprintResources/StandardMacros.FlipFlop`
      (:`A`
        (`AeroPhysicsComponent.SetAeroFlapControl` _aerophysicscomponent 1.0))
      (:`B`
        (`AeroPhysicsComponent.SetAeroFlapControl` _aerophysicscomponent 0.0)))))

(event `InputAxis|Thruster`
  (params (AxisValue :type "Float (single-precision)"))
  (`AeroPhysicsComponent.SetAddThruster` (`self.AeroPhysicsComponent`) AxisValue))

(event `InputAction|WheelRetreat`
  (params (Key :type "Key Structure"))
  (:`Pressed`
    (`AeroPhysicsComponent.SetWheelsRetreated` (`self.AeroPhysicsComponent`) (not (`AeroPhysicsComponent.GetIsWheelsRetreated` (`self.AeroPhysicsComponent`))))))

(event `self.ReceiveBeginPlay`
  (`parent.ReceiveBeginPlay`)
  (bind _returnvalue (`|CreateWidget` "/Game/FighterJet/Fighter.Fighter_C" (`GameplayStatics.GetPlayerController` 0)))
  (set `/Game/FighterJet/Fighter.Fighter` self _returnvalue)
  (`UserWidget.AddToViewport` _returnvalue 0))

(fn `UserConstructionScript`
  (`parent.UserConstructionScript`))