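; Player-controlled F-15E fighter jet Blueprint that routes axis input to flight and camera controls and sets up its on-screen widget.
; Thruster, wheel steering and brake axes feed straight into AeroPhysicsComponent, while look and turn axes drive controller pitch and yaw.
; On BeginPlay it creates the Fighter widget for the first player, hands it a self reference and adds it to the viewport.
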(event `InputAxis|LookUp`
  (params (AxisValue :type "Float (single-precision)"))
  (`self.AddControllerPitchInput` AxisValue))

(event `InputAxis|TurnRight`
  (params (AxisValue :type "Float (single-precision)"))
  (`self.AddControllerYawInput` AxisValue))

(event `InputAxis|WheelTurn`
  (params (AxisValue :type "Float (single-precision)"))
  (`AeroPhysicsComponent.SetSteeringWheels` (`self.AeroPhysicsComponent`) AxisValue))

(event `InputAxis|Brake`
  (params (AxisValue :type "Float (single-precision)"))
  (`AeroPhysicsComponent.SetWheelsBrake` (`self.AeroPhysicsComponent`) AxisValue))

(event `InputAxis|Thruster`
  (params (AxisValue :type "Float (single-precision)"))
  (`AeroPhysicsComponent.SetAddThruster` (`self.AeroPhysicsComponent`) AxisValue))

(event `self.ReceiveBeginPlay`
  (`parent.ReceiveBeginPlay`)
  (bind _returnvalue (`|CreateWidget` "/Game/FighterJet/Fighter.Fighter_C" (`GameplayStatics.GetPlayerController` 0)))
  (set `/Game/FighterJet/Fighter.Fighter` self _returnvalue)
  (`UserWidget.AddToViewport` _returnvalue 0))

(fn `UserConstructionScript`
  (`parent.UserConstructionScript`))